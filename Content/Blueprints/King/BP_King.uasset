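; BP_King is the king character, who plays a laugh or "urk" reaction depending on a Happy flag.
; KingReact picks one of two random variants for that mood and, on a laugh, triggers PublicReact on every BP_Gradin in the level.
; It returns to the looping idle shortly after the animation's length has elapsed, with PlayingReact blocking new reactions until then.
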(event Custom|KingReact
  (params (Happy :type Boolean))
  (bind _returnvalue (Math|Random|RandomBool))
  (bind _skeletalmesh (Variables|Default|GetSkeletalMesh))
  (if (not (Variables|Default|GetPlayingReact))
    (Variables|Default|SetPlayingReact true)
    (bind _output_get (Variables|Default|SetAnimationPlaying (Math|Integer|SelectInt (Math|Integer|SelectInt 0 1 _returnvalue) (Math|Integer|SelectInt 2 3 _returnvalue) Happy)))
    (bind _outactors (Actor|GetAllActorsOfClass "/Game/Blueprints/Decor_Animated/BP_Gradin.BP_Gradin_C"))
    (for _array_element _outactors
      (if (< _output_get 2)
        (Default|PublicReact _array_element)))
    (Components|Animation|PlayAnimation _skeletalmesh (Utilities|Select :Index _output_get :Option%200 "/Game/King_3D/Anim/ANIM_king_laught_A.ANIM_king_laught_A" :Option%201 "/Game/King_3D/Anim/ANIM_king_laught_B.ANIM_king_laught_B" :Option%202 "/Game/King_3D/Anim/ANIM_king_urk_A.ANIM_king_urk_A" :Option%203 "/Game/King_3D/Anim/ANIM_king_urk_B.ANIM_king_urk_B") false)
    (Utilities|FlowControl|Delay (+ (Animation|GetPlayLength (.animtoplay (Variables|/Script/Engine.SkeletalMeshComponent|GetAnimationData _skeletalmesh))) 0.2))
    (Components|Animation|PlayAnimation (Variables|Default|GetSkeletalMesh) "/Game/King_3D/Anim/ANIM_king_idle.ANIM_king_idle" true)
    (Variables|Default|SetPlayingReact false)))

(fn ConstructionScript)