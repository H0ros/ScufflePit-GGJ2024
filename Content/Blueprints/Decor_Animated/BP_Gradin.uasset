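; BP_Gradin is an animated decor grandstand that reacts with a burst of crowd excitement.
; Public_React speeds up the SKGradin animation, swaps its material and plays a 2D crowd sound, then reverts to slow playback and the normal material after a short delay.
; The construction script gives each lettered component a random material from the SturctMat struct, though its random range never selects InstD.
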(event Custom|Public_React
  (bind _sk_gradin (Variables|Default|GetSK_Gradin))
  (Components|Timeline|SetPlayRate _sk_gradin 3.0)
  (Rendering|Material|SetMaterial _sk_gradin 0 "/Game/Decor_3D/INST_Gradin1.INST_Gradin1")
  (Audio|PlaySound2D "/Game/Sound/CUE_Crowd.CUE_Crowd" 1.0 1.0 0.0 0 0)
  (Utilities|FlowControl|Delay 2.0)
  (Components|Timeline|SetPlayRate _sk_gradin 0.5)
  (Rendering|Material|SetMaterial _sk_gradin 0 "/Game/Decor_3D/INST_Gradin.INST_Gradin"))

(fn ConstructionScript
  (bind _sturct_mat (Variables|Default|GetSturct%20Mat))
  (bind (_insta _instb _instc _instd) (Utilities|Struct|BreakSTRUCT_Mt _sturct_mat))
  (for _array_element (Utilities|Array|MakeArray (Variables|Default|GetO) (Variables|Default|GetB) (Variables|Default|GetC) (Variables|Default|GetE) (Variables|Default|GetF) (Variables|Default|GetG) (Variables|Default|GetH) (Variables|Default|GetI) (Variables|Default|GetJ) (Variables|Default|GetK) (Variables|Default|GetL) (Variables|Default|GetM) (Variables|Default|GetN) (Variables|Default|GetA) (Variables|Default|GetP) (Variables|Default|GetQ) (Variables|Default|GetR) (Variables|Default|GetS) (Variables|Default|GetT) (Variables|Default|GetU) (Variables|Default|GetV) (Variables|Default|GetW) (Variables|Default|GetX) (Variables|Default|GetY) (Variables|Default|GetZ) (Variables|Default|GetAZ))
    (Rendering|Material|SetMaterial _array_element 0 (Utilities|Select :Index (Math|Random|RandomInteger 3) :Option%200 _insta :Option%201 _instb :Option%202 _instc :Option%203 _instd))))