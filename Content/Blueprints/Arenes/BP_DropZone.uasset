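; BP_DropZone is an arena kill volume that handles players and boxes falling out of the Scuffle Pit.
; When a player overlaps its box, the game mode deducts score from them and credits their last hitter, if valid.
; It then plays a fall voice cue and respawns the player after a three-second timer.
; Overlapping BP_Box actors respawn immediately.
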(event OnComponentBeginOverlap(Box)
  (params (OverlappedComponent :type Primitive%20Component%20Object%20Reference) (OtherActor :type Actor%20Object%20Reference) (OtherComp :type Primitive%20Component%20Object%20Reference) (OtherBodyIndex :type Integer) (bFromSweep :type Boolean) (SweepResult :type Hit%20Result%20Structure%20%28by%20ref%29))
  (bind _gmref (Variables|Default|GetGMRef))
  (bind _asbp_base_player (Utilities|Casting|CastToBP_BasePlayer OtherActor)
    (:then
      (Default|UpdateScore _gmref (Variables|/Game/Blueprints/Players/BP_BasePlayer.BP_BasePlayer_C|GetControllerID _asbp_base_player) false "NewEnumerator0")
      (bind _lasthitter (Variables|/Game/Blueprints/Players/BP_BasePlayer.BP_BasePlayer_C|GetLastHitter _asbp_base_player)
        (:then
          (Default|UpdateScore _gmref (Variables|/Game/Blueprints/Players/BP_BasePlayer.BP_BasePlayer_C|GetControllerID _lasthitter) true "NewEnumerator0"))
        (:else
          _))
      (Audio|PlaySoundatLocation "/Game/Sound/CUE_Vox_Fall.CUE_Vox_Fall" (Transformation|GetActorLocation _asbp_base_player) "0, 0, 0" 1.0 1.0 0.0 0 0 _asbp_base_player 0)
      (Utilities|Time|SetTimerbyFunctionName _asbp_base_player "Respawn" 3.0))
    (:CastFailed
      (bind _asbp_box (Utilities|Casting|CastToBP_Box OtherActor))
      (Default|Respawn _asbp_box))))

(event EventBeginPlay
  (bind _asbp_gm_scuffle_pit (Utilities|Casting|CastToBP_GM_ScufflePit (Game|GetGameMode)))
  (Variables|Default|SetGMRef _asbp_gm_scuffle_pit))

(fn ConstructionScript)