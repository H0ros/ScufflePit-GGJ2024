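; BP_Floor is an arena floor piece that can rise into view, retract, drop away and reset.
; DisplayFloor plays the MoveUp timeline at a randomized rate to offset the mesh vertically, and HideFloor reverses it.
; DropFloor enables physics, ignores Pawn collision and flags the piece as fallen.
; ResetFloor hides it, then after a delay stops physics, reattaches the mesh and snaps it to its lowered position.
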(event Custom|DropFloor
  (bind _sm_floor (Variables|Default|GetSM_Floor))
  (Physics|SetSimulatePhysics _sm_floor true)
  (Collision|SetCollisionResponsetoChannel _sm_floor "ECC_Pawn" "ECR_Ignore")
  (Variables|Default|SetFallen true))

(event Custom|DisplayFloor
  (Components|Timeline|SetPlayRate (Variables|Default|GetMoveUp) (Math|Random|RandomFloatinRange 0.7 1.3))
  (bind _zoffset (Timeline|MoveUp PlayFromStart)
    (:Update
      (Transformation|SetRelativeLocation (Variables|Default|GetSM_Floor) (Math|Vector|MakeVector 0.0 0.0 (* _zoffset -7e+02)) false false))
    (:Finished
      (Variables|Default|SetFallen false))))

(event Custom|HideFloor
  (bind _zoffset (Timeline|MoveUp ReverseFromEnd)
    (:Update
      (Transformation|SetRelativeLocation (Variables|Default|GetSM_Floor) (Math|Vector|MakeVector 0.0 0.0 (* _zoffset -7e+02)) false false))
    (:Finished
      (Variables|Default|SetFallen false))))

(event Custom|ResetFloor
  (bind _sm_floor (Variables|Default|GetSM_Floor))
  (CallFunction|HideFloor)
  (Utilities|FlowControl|Delay 1.0)
  (Physics|SetSimulatePhysics _sm_floor false)
  (Variables|Default|SetFallen false)
  (Transformation|AttachComponentToComponent _sm_floor (Variables|Default|GetDefaultSceneRoot) "None" "SnapToTarget" "SnapToTarget" "KeepWorld" true)
  (Transformation|SetRelativeLocation _sm_floor "0.000000,0.000000,-700.000000" false false))

(fn ConstructionScript)