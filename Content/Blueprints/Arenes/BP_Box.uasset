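; Physics box for the ScufflePit arenas that knocks players away and scores for the player who owns it.
; On BeginPlay it gets a random mass, shown as emissive color on a dynamic material.
; Hitting a player applies a velocity-scaled push, sets the owner as temporary last hitter, updates the game mode score and clears ownership.
; Other hits clear ownership after a delay, non-floor impacts play debounced sounds, and Respawn resets the box.
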(event OnComponentHit(SM_Box)
  (params (HitComponent :type Primitive%20Component%20Object%20Reference) (OtherActor :type Actor%20Object%20Reference) (OtherComp :type Primitive%20Component%20Object%20Reference) (NormalImpulse :type Vector :default "0, 0, 0") (Hit :type Hit%20Result%20Structure%20%28by%20ref%29))
  (bind _asbp_base_player (Utilities|Casting|CastToBP_BasePlayer OtherActor)
    (:then
      (bind _owningplayer (Variables|Default|GetOwningPlayer)
        (:then
          (Variables|/Game/Blueprints/Players/BP_BasePlayer.BP_BasePlayer_C|SetLastHitter _asbp_base_player _owningplayer)
          (Utilities|Time|SetTimerbyFunctionName _asbp_base_player "ResetLastHitter" 3.0)
          (Default|PlayersHit _asbp_base_player (* (- (Transformation|GetActorLocation _asbp_base_player) (Transformation|GetActorLocation)) (/ (Math|Vector|VectorLength (Transformation|GetComponentVelocity (Variables|Default|GetSM_Box))) 2e+03)))
          (Default|UpdateScore (Variables|Default|GetGMRef) (Variables|/Game/Blueprints/Players/BP_BasePlayer.BP_BasePlayer_C|GetControllerID (Variables|Default|GetOwningPlayer)) true "NewEnumerator1")
          (Variables|Default|SetOwningPlayer 0))
        (:else)))
    (:CastFailed
      (Variables|Default|GetOwningPlayer
        (:then
          (Utilities|FlowControl|Delay 1.0)
          (Variables|Default|SetOwningPlayer 0))
        (:else)))))

(event EventBeginPlay
  (bind _asbp_gm_scuffle_pit (Utilities|Casting|CastToBP_GM_ScufflePit (Game|GetGameMode)))
  (Variables|Default|SetGMRef _asbp_gm_scuffle_pit)
  (bind _output_get (Variables|Default|SetNewMass (Math|Random|RandomFloatinRange 1e+01 1e+02)))
  (Class|PrimitiveComponent|SetMassOverrideinKg (Variables|Default|GetSM_Box) "None" _output_get true)
  (Rendering|Material|SetVectorParameterValue (Variables|Default|GetDynamicMaterialInstance) "Emissive Color" (select (> (Variables|Default|GetNewMass) 7e+01) "(R=1.000000,G=0.000000,B=0.000000,A=1.000000)" (select (> (Variables|Default|GetNewMass) 4e+01) "(R=1.000000,G=0.000000,B=1.000000,A=1.000000)" "(R=0.000000,G=0.000000,B=1.000000,A=1.000000)")) :!class /Script/Engine.MaterialInstanceDynamic))

(event Collision|EventHit
  (params (MyComp :type Primitive%20Component%20Object%20Reference) (Other :type Actor%20Object%20Reference) (OtherComp :type Primitive%20Component%20Object%20Reference) (bSelfMoved :type Boolean) (HitLocation :type Vector :default "0, 0, 0") (HitNormal :type Vector :default "0, 0, 0") (NormalImpulse :type Vector :default "0, 0, 0") (Hit :type Hit%20Result%20Structure%20%28by%20ref%29))
  (bind _sound (Variables|Default|GetSound))
  (if (not (Utilities|String|Contains (Utilities|String|ToString(Object) Other) "floor"))
    (Utilities|FlowControl|Sequence
      (:then_0
        (Utilities|FlowControl|DoOnce false :!label _label
          (:Completed
            (Utilities|IsValid _sound
              (:Is%20Valid
                (Audio|SpawnSoundatLocation _sound (Transformation|GetWorldLocation (Variables|Default|GetSM_Box)) "0, 0, 0" 1.0 1.0 0.0 0 0))))))
      (:then_1
        (Utilities|FlowControl|RetriggerableDelay 0.1)
        (goto _label Reset)))))

(fn ConstructionScript
  (bind _returnvalue (Rendering|Material|CreateDynamicMaterialInstance "/Game/Decor_3D/INST_Cube.INST_Cube" "None" "None" :!class /Script/Engine.KismetMaterialLibrary))
  (bind _output_get (Variables|Default|SetDynamicMaterialInstance _returnvalue))
  (Rendering|Material|SetMaterial (Variables|Default|GetSM_Box) 0 _output_get))

(fn Respawn
  (bind _sm_box (Variables|Default|GetSM_Box))
  (Class|PrimitiveComponent|SetAllPhysicsLinearVelocity _sm_box "0, 0, 0" false)
  (Transformation|SetWorldLocation _sm_box (Transformation|GetWorldLocation (Variables|Default|GetRoot)) false false)
  (Variables|Default|SetOwningPlayer 0))