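; BP_EnergyBall is an arena hazard that homes in on players and knocks them back.
; StartBehavior gathers players, starts a looping retarget timer and ramps speed through the EnterArena timeline.
; Tick moves and turns it toward its target with clamped height, scaling Niagara particle lifetime with speed.
; Overlaps trigger speed-scaled knockback, penalize the victim's score and credit their last hitter.
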(event Custom|StartBehavior
  (bind _outactors (Actor|GetAllActorsOfClass "/Game/Blueprints/Players/BP_BasePlayer.BP_BasePlayer_C"))
  (Variables|Default|SetPlayers _outactors)
  (Variables|Default|SetCanMove true)
  (bind _returnvalue (Utilities|Time|SetTimerbyEvent (EventDispatchers|CreateEvent :!event Custom|CheckNearestActor) 2.0 true))
  (Variables|Default|SetTargetTimer _returnvalue)
  (bind _ballspeed (Timeline|EnterArena PlayFromStart)
    (:Update
      (Variables|Default|SetMovementSpeed _ballspeed))))

(event Custom|CheckNearestActor
  (Variables|Default|SetTarget (.ReturnValue (Actor|FindNearestActor (Transformation|GetActorLocation) (Variables|Default|GetPlayers)))))

(event EventTick
  (params (DeltaSeconds :type Float%20%28single-precision%29))
  (bind _niagara (Variables|Default|GetNiagara))
  (bind _movementspeed (Variables|Default|GetMovementSpeed))
  (bind _returnvalue (/ _movementspeed 1.5e+02))
  (bind _returnvalue_2 (* _returnvalue 0.3))
  (if (Variables|Default|GetCanMove)
    (Utilities|FlowControl|Sequence
      (:then_0
        (CallFunction|FollowTarget))
      (:then_1
        (CallFunction|CheckOverlappingPlayers))
      (:then_2
        (Niagara|SetNiagaraVariable(Float) _niagara "User.LifetimeMin" _returnvalue_2)
        (Niagara|SetNiagaraVariable(Float) _niagara "User.LifetimeMax" (* _returnvalue_2 2.0))))
    (else
      (Niagara|SetNiagaraVariable(Float) _niagara "User.LifetimeMin" 0.0)
      (Niagara|SetNiagaraVariable(Float) _niagara "User.LifetimeMax" 0.0))))

(fn ConstructionScript
  (Variables|Default|SetInitLocation (Transformation|GetActorLocation)))

(fn CheckOverlappingPlayers
  (bind _gmref (Variables|Default|GetGMRef))
  (for _array_element (Collision|GetOverlappingActors "/Game/Blueprints/Players/BP_BasePlayer.BP_BasePlayer_C" :!class /Script/Engine.Actor)
    (bind _asbp_base_player (Utilities|Casting|CastToBP_BasePlayer _array_element))
    (if (Variables|/Game/Blueprints/Players/BP_BasePlayer.BP_BasePlayer_C|GetCanBeKnockedBack _asbp_base_player)
      (Default|PlayersHit _asbp_base_player (* (select (Math|Vector|VectorIsNearlyZero (- (Transformation|GetActorLocation _asbp_base_player) (Transformation|GetActorLocation)) 1e+01) (* (Transformation|GetActorForwardVector) -1e+02) (- (Transformation|GetActorLocation _asbp_base_player) (Transformation|GetActorLocation))) (/ (Variables|Default|GetMovementSpeed) 1.5e+02)))
      (Default|UpdateScore _gmref (Variables|/Game/Blueprints/Players/BP_BasePlayer.BP_BasePlayer_C|GetControllerID _asbp_base_player) false "NewEnumerator2")
      (bind _lasthitter (Variables|/Game/Blueprints/Players/BP_BasePlayer.BP_BasePlayer_C|GetLastHitter _asbp_base_player)
        (:then
          (Default|UpdateScore _gmref (Variables|/Game/Blueprints/Players/BP_BasePlayer.BP_BasePlayer_C|GetControllerID _lasthitter) true "NewEnumerator2"))
        (:else)))))

(fn FollowTarget
  (bind _target (Variables|Default|GetTarget)
    (:then
      (Transformation|SetActorLocationAndRotation (Math|Interpolation|VInterptoConstant (Transformation|GetActorLocation) (Math|Vector|MakeVector (.X (Math|Vector|BreakVector (Transformation|GetActorLocation _target))) (.Y (Math|Vector|BreakVector (Transformation|GetActorLocation _target))) (Math|Float|Clamp(Float) (.Z (Math|Vector|BreakVector (Transformation|GetActorLocation _target))) 2e+02 1e+03)) (Utilities|Time|GetWorldDeltaSeconds) (Variables|Default|GetMovementSpeed)) (Class|KismetMathLibrary|RInterptoConstant (Transformation|GetActorRotation) (Math|Rotator|FindLookatRotation (Transformation|GetActorLocation) (Transformation|GetActorLocation _target)) (Utilities|Time|GetWorldDeltaSeconds) (Variables|Default|GetRotationSpeed)) true))
    (:else)))