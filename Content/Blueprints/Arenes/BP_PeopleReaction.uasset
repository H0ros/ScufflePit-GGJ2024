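; BP_PeopleReaction is the Scuffle Pit arena crowd, which punishes players who stay inactive.
; A one-second looping timer compares each player's inactivity to a limit while the round runs, then reacts by arena type.
; Fall drops floors around the player, Throw launches a physics box at them, and Run spawns energy balls, capped by the round timer value.
; Reactions play sounds and reset or reduce the inactivity time.
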(event Custom|CheckInactivity
  (bind _arrow (Variables|Default|GetArrow))
  (bind _returnvalue (Transformation|GetWorldLocation _arrow))
  (if (Utilities|Time|IsTimerActivebyHandle (Variables|/Game/Blueprints/Players/BP_GM_ScufflePit.BP_GM_ScufflePit_C|GetRoundTimer (Variables|Default|GetGMRef)))
    (for _array_element (Variables|Default|GetPlayers)
      (if (> (Variables|/Game/Blueprints/Players/BP_BasePlayer.BP_BasePlayer_C|GetInactivityTime _array_element) (Variables|Default|GetInactivityLimit))
        (switch Utilities|FlowControl|Switch|SwitchonEnum_ArenaType (Variables|/Game/Blueprints/Players/BP_GM_ScufflePit.BP_GM_ScufflePit_C|GetArenaType (Variables|Default|GetGMRef))
          (:NewEnumerator0
            (bind (_outhits _returnvalue_2) (Collision|MultiSphereTraceByChannel (Transformation|GetActorLocation _array_element) (Transformation|GetActorLocation _array_element) 1e+02 "TraceTypeQuery1" false 0 "None"))
            (if _returnvalue_2
              (for _array_element_2 _outhits
                (bind _asbp_floor (Utilities|Casting|CastToBP_Floor (.HitActor (Collision|BreakHitResult _array_element_2))))
                (Default|DropFloor _asbp_floor))
              (Variables|/Game/Blueprints/Players/BP_BasePlayer.BP_BasePlayer_C|SetInactivityTime _array_element 0)
              (Audio|PlaySound2D "/Game/Sound/CUE_Crowd.CUE_Crowd" 1.0 1.0 0.0 0 0)))
          (:NewEnumerator1
            (Audio|PlaySound2D "/Game/Sound/CUE_Crowd.CUE_Crowd" 1.0 1.0 0.0 0 0)
            (bind _returnvalue_3 (Game|SpawnActorfromClass "/Game/Blueprints/Arenes/BP_Box.BP_Box_C" (Math|Transform|MakeTransform (+ _returnvalue (* (Math|Vector|GetForwardVector (Math|Rotator|FindLookatRotation _returnvalue (Transformation|GetActorLocation _array_element))) 1.5e+02)) (Math|Rotator|FindLookatRotation _returnvalue (Transformation|GetActorLocation _array_element))) "Undefined" "MultiplyWithRoot" 0 true 0))
            (Physics|SetSimulatePhysics (Variables|/Game/Blueprints/Arenes/BP_Box.BP_Box_C|GetSM_Box _returnvalue_3) true)
            (Physics|AddImpulse (Variables|/Game/Blueprints/Arenes/BP_Box.BP_Box_C|GetSM_Box _returnvalue_3) (* (Math|Vector|GetForwardVector (Math|Rotator|FindLookatRotation _returnvalue (Transformation|GetActorLocation _array_element))) 2e+05) "None" false)
            (Audio|PlaySound2D "/Game/Sound/CUE_Throw.CUE_Throw" 1.0 1.0 0.0 0 0)
            (Utilities|FlowControl|Delay 0.5)
            (Variables|/Game/Blueprints/Players/BP_BasePlayer.BP_BasePlayer_C|SetInactivityTime _array_element (- (Variables|/Game/Blueprints/Players/BP_BasePlayer.BP_BasePlayer_C|GetInactivityTime _array_element) 5)))
          (:NewEnumerator2
            (bind _outactors (Actor|GetAllActorsOfClass "/Game/Blueprints/Arenes/BP_EnergyBall.BP_EnergyBall_C"))
            (if (< (Utilities|Array|Length _outactors) (/ (Variables|/Game/Blueprints/Players/BP_GM_ScufflePit.BP_GM_ScufflePit_C|GetTimerValue (Variables|Default|GetGMRef)) 15))
              (bind _returnvalue_4 (Actor|GetActorOfClass "/Game/Blueprints/Arenes/BP_BallSPawner.BP_BallSPawner_C"))
              (Default|SpawnBall _returnvalue_4)
              (Audio|PlaySound2D "/Game/Sound/CUE_Crowd.CUE_Crowd" 1.0 1.0 0.0 0 0)
              (Audio|PlaySound2D "/Game/Sound/CUE_DarkMatter_Hit.CUE_DarkMatter_Hit" 1.0 1.0 0.0 0 0)
              (Variables|/Game/Blueprints/Players/BP_BasePlayer.BP_BasePlayer_C|SetInactivityTime _array_element 0))))))))

(event EventBeginPlay
  (Utilities|FlowControl|Delay 8.0)
  (bind _outactors (Actor|GetAllActorsOfClass "/Game/Blueprints/Players/BP_BasePlayer.BP_BasePlayer_C"))
  (Variables|Default|SetPlayers _outactors)
  (bind _asbp_gm_scuffle_pit (Utilities|Casting|CastToBP_GM_ScufflePit (Game|GetGameMode)))
  (Variables|Default|SetGMRef _asbp_gm_scuffle_pit)
  (Utilities|Time|SetTimerbyEvent (delegate Custom|CheckInactivity) 1.0 true))

(fn ConstructionScript)