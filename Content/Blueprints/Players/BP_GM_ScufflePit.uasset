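; Game mode for Scuffle Pit that sets up the shared gameplay camera and local players at BeginPlay.
; It blacks out the screen, switches the first player's view to the placed BP_GameplayCamera and fades in, or prints an error if none exists.
; It then reads the player count from the game instance, creating each additional local player with a controller ID and loading input mapping contexts for all.
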(event EventBeginPlay
  (Utilities|FlowControl|Sequence
    (:then_0
      (bind _asbp_gi_scuffle_pit (Utilities|Casting|CastToBP_GI_ScufflePit (Game|GetGameInstance)))
      (Variables|Default|SetAs%20BP%20GI%20Scuffle%20Pit _asbp_gi_scuffle_pit))
    (:then_1
      (CallFunction|CameraSetup))
    (:then_2
      (CallFunction|HandlePlayers))))

(fn ConstructionScript)

(fn CameraSetup
  (CameraFades|StartCameraFade :self (Game|GetPlayerCameraManager 0) :FromAlpha 1.0 :ToAlpha 1.0 :Duration 1.0 :bHoldWhenFinished true)
  (bind _returnvalue (Actor|GetActorOfClass "/Game/Blueprints/BP_GameplayCamera.BP_GameplayCamera_C"))
  (Utilities|IsValid _returnvalue
    (:Is%20Valid
      (Game|Player|SetViewTargetwithBlend (Game|GetPlayerController 0) _returnvalue 0.0 "VTBlend_Linear" 0.0 false)
      (CameraFades|StartCameraFade :self (Game|GetPlayerCameraManager 0) :FromAlpha 1.0 :Duration 5.0 :bHoldWhenFinished true))
    (:Is%20Not%20Valid
      (Development|PrintString "Please add a Gameplay Camera to the scene" true true "(R=1.000000,G=0.000000,B=0.000000,A=1.000000)" 1e+01))))

(fn HandlePlayers
  (for _index (range 0 (- (Variables|/Game/Blueprints/Players/BP_GI_ScufflePit.BP_GI_ScufflePit_C|GetPlayersNB (Variables|Default|GetAs%20BP%20GI%20Scuffle%20Pit)) 1))
    (switch int _index
      (:Default
        (bind _returnvalue (Class|GameplayStatics|CreatePlayer _index))
        (bind _asbp_pc_player (Utilities|Casting|CastToBP_PC_Player _returnvalue))
        (Default|LoadMappingContext _asbp_pc_player)
        (Variables|/Game/Blueprints/Players/BP_PC_Player.BP_PC_Player_C|SetControllerID _asbp_pc_player _index))
      (:0
        (bind _asbp_pc_player_2 (Utilities|Casting|CastToBP_PC_Player (Game|GetPlayerController 0)))
        (Default|LoadMappingContext _asbp_pc_player_2)))))