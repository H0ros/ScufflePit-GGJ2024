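; BP_PC_Player is a player controller that gives each possessed player character a distinct color.
; On possess, it casts the pawn to BP_BasePlayer and sets its dynamic material's hue parameter to a random value within a band chosen by controller ID, keeping four players' hues separate.
; A separate LoadMappingContext function adds the IMC_Players Enhanced Input context, though nothing in this Blueprint calls it.
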(event EventPossess
  (params (PossessedPawn :type Pawn%20Object%20Reference))
  (bind _self self)
  (bind _returnvalue (Class|GameplayStatics|GetPlayerControllerID _self))
  (bind _asbp_base_player (Utilities|Casting|CastToBP_BasePlayer PossessedPawn))
  (Rendering|Material|SetScalarParameterValue (Variables|/Game/Blueprints/Players/BP_BasePlayer.BP_BasePlayer_C|GetDynamicMaterial _asbp_base_player) "Hue_Tex_Var" (Math|Random|RandomFloatinRange (Utilities|Select :Index _returnvalue :Option%200 0.0 :Option%201 0.22 :Option%202 0.44 :Option%203 0.66) (Utilities|Select :Index _returnvalue :Option%200 0.21 :Option%201 0.43 :Option%202 0.65 :Option%203 0.87)) :!class /Script/Engine.MaterialInstanceDynamic))

(fn ConstructionScript)

(fn LoadMappingContext
  (Input|AddMappingContext (PlayerController|LocalPlayerSubsystems|GetEnhancedInputLocalPlayerSubsystem) "/Game/Blueprints/Players/Inputs/IMC_Players.IMC_Players" 0 "(bIgnoreAllPressedKeysUntilRelease=True,bForceImmediately=False,bNotifyUserSettings=False)"))